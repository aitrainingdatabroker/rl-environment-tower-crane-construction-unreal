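; Keyboard controller for a construction crane made of separate slew, trolley, hook and cable actors.
; BeginPlay enables player input and seeds trolley and hook positions.
; Tick polls key states: J/L rotate the slew, I/K move the trolley and R/F raise or lower the hook, both within clamped limits.
; The cable is a scaled actor, positioned at half the hook's offset and stretched in Z to match the drop.
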(event `self.ReceiveBeginPlay`
  (`self.EnableInput` self (`GameplayStatics.GetPlayerController` 0))
  (set `self.TrolleyX` 1400.0)
  (set `self.HookZ` -800.0))

(event `self.ReceiveTick`
  (params (DeltaSeconds :type "Float (single-precision)"))
  (bind _returnvalue (`GameplayStatics.GetPlayerController` 0))
  (bind _cable (`self.Cable`))
  (bind _returnvalue_2 (`KismetMathLibrary.FClamp` (+ (`self.TrolleyX`) (* (- (`KismetMathLibrary.SelectFloat` 1.0 0.0 (`PlayerController.IsInputKeyDown` _returnvalue "I")) (`KismetMathLibrary.SelectFloat` 1.0 0.0 (`PlayerController.IsInputKeyDown` _returnvalue "K"))) (* 400.0 DeltaSeconds))) 300.0 3400.0))
  (bind _returnvalue_3 (`KismetMathLibrary.FClamp` (+ (`self.HookZ`) (* (- (`KismetMathLibrary.SelectFloat` 1.0 0.0 (`PlayerController.IsInputKeyDown` _returnvalue "R")) (`KismetMathLibrary.SelectFloat` 1.0 0.0 (`PlayerController.IsInputKeyDown` _returnvalue "F"))) (* 300.0 DeltaSeconds))) -2650.0 -150.0))
  (`self.K2_AddActorWorldRotation` (`self.Slew`) (`KismetMathLibrary.MakeRotator` 0.0 0.0 (* (- (`KismetMathLibrary.SelectFloat` 1.0 0.0 (`PlayerController.IsInputKeyDown` _returnvalue "L")) (`KismetMathLibrary.SelectFloat` 1.0 0.0 (`PlayerController.IsInputKeyDown` _returnvalue "J"))) (* 30.0 DeltaSeconds))) false false)
  (set `self.TrolleyX` _returnvalue_2)
  (`self.K2_SetActorRelativeLocation` (`self.Trolley`) (`KismetMathLibrary.MakeVector` _returnvalue_2 0.0 -40.0) false false)
  (set `self.HookZ` _returnvalue_3)
  (`self.K2_SetActorRelativeLocation` (`self.Hook`) (`KismetMathLibrary.MakeVector` 0.0 0.0 _returnvalue_3) false false)
  (`self.K2_SetActorRelativeLocation` _cable (`KismetMathLibrary.MakeVector` 0.0 0.0 (* _returnvalue_3 0.5)) false false)
  (`self.SetActorRelativeScale3D` _cable (`KismetMathLibrary.MakeVector` 0.04 0.04 (/ (- 0.0 _returnvalue_3) 100.0))))

(fn `UserConstructionScript`)